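; BP_Fog_Card is a placeable fog card: a scalable plane with tunable panning, intensity, fresnel, depth fade, distance fading and tint.
; The construction script scales the plane and picks a random or non-random movement material.
; It packs the settings into three Custom Primitive Data vectors, giving per-card variation without dynamic material instances.
; It has no runtime logic, as the event graph and NewFunction are empty.
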(event EventBeginPlay)

(event Collision|EventActorBeginOverlap
  (params (OtherActor :type Actor%20Object%20Reference)))

(event EventTick
  (params (DeltaSeconds :type Float%20%28single-precision%29)))

(fn ConstructionScript
  (bind _tint (Variables|Default|Gettint))
  (bind _plane (Variables|Default|GetPlane))
  (Transformation|SetRelativeScale3D _plane (Math|Vector|MakeVector (Variables|Default|GetPlane%20scale%20X) (Variables|Default|GetPlane%20scale%20Y) 1.0))
  (Rendering|Material|SetMaterial _plane 0 (select (Variables|Default|Getuse%20Random%20Direction) (Variables|Material|Getfog%20material_RandomMovement) (Variables|Material|Getfog%20material_NoRandomMovement)))
  (Rendering|Material|SetDefaultCustomPrimitiveDataVector4 _plane 0 (Math|Vector4|MakeVector4 (Variables|Default|GetX%20panning%20speed) (Variables|Default|GetY%20panning%20speed) (Variables|Default|Getoverall%20intensity%20exponent) (Variables|Default|Getoverall%20intensity%20multiplier)))
  (Rendering|Material|SetDefaultCustomPrimitiveDataVector4 _plane 4 (Math|Vector4|MakeVector4 (Variables|Default|Getfresnel%20power) (Variables|Default|Getdepth%20fade) (Variables|Default|Getfog%20thickest%20distance) (Variables|Default|Getgap%20closing%20transition%20distance)))
  (Rendering|Material|SetDefaultCustomPrimitiveDataVector4 _plane 8 (Math|Vector4|MakeVector4 (.r _tint) (.g _tint) (.b _tint) (Variables|Default|Getdetail%20intensity%20exponent))))

(fn NewFunction)